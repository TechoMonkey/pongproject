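; Pong-style ball actor that bounces off player and enemy paddles and walls by editing its ProjectileMovement velocity.
; Paddle overlaps add randomized vertical spin biased by the paddle's MoveDirection, then flip X velocity; wall overlaps flip Z.
; A Tick-driven timer limits horizontal flips to one-second intervals, but spin applies regardless.
; Wall bounces reset that shared timer with a zero threshold, so they can block a following paddle flip.
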(event EventBeginPlay)

(event EventTick
  (params (DeltaSeconds :type Float%20%28single-precision%29))
  (Variables|Default|SettimeSinceReversed (+ DeltaSeconds (Variables|Default|GettimeSinceReversed))))

(event Collision|EventActorBeginOverlap
  (params (OtherActor :type Actor%20Object%20Reference))
  (bind _asplayer_paddle (Utilities|Casting|CastToPlayerPaddle OtherActor)
    (:then
      (CallFunction|HandleBounce (Variables|/Game/Blueprints/PlayerPaddle.PlayerPaddle_C|GetMoveDirection _asplayer_paddle)))
    (:CastFailed
      (bind _asenemy_paddle_2 (Utilities|Casting|CastToEnemyPaddle2 OtherActor)
        (:then
          (CallFunction|HandleBounce (Variables|/Game/Blueprints/EnemyPaddle2.EnemyPaddle2_C|GetMoveDirection _asenemy_paddle_2)))
        (:CastFailed
          (Utilities|Casting|CastToWall OtherActor)
          (CallFunction|ReverseVertical))))))

(fn ConstructionScript)

(fn HandleBounce
  (params (Selection :type Integer))
  (bind _returnvalue (Math|Random|RandomFloatinRange -5e+01 5e+01))
  (switch int Selection
    (:-1
      (CallFunction|AddSpin (+ _returnvalue -125.0)))
    (:0
      (CallFunction|AddSpin (Math|Random|RandomFloatinRange -15.0 15.0)))
    (:1
      (CallFunction|AddSpin (+ _returnvalue 125.0))))
  (CallFunction|ReverseHoriz))

(fn AddSpin
  (params (Z :type Float%20%28single-precision%29))
  (Variables|/Script/Engine.MovementComponent|SetVelocity (Variables|Default|GetProjectileMovement) (+ (Math|Vector|MakeVector 0.0 0.0 Z) (Variables|/Script/Engine.MovementComponent|GetVelocity (Variables|Default|GetProjectileMovement)))))

(fn ReverseHoriz
  (bind _returnvalue (Transformation|GetVelocity))
  (bind (_x _y _z) (Math|Vector|BreakVector _returnvalue))
  (if (>= (Variables|Default|GettimeSinceReversed) 1.0)
    (Variables|/Script/Engine.MovementComponent|SetVelocity (Variables|Default|GetProjectileMovement) (Math|Vector|MakeVector (* -1 (+ _x 0.0)) _y _z))
    (Variables|Default|SettimeSinceReversed 0.0)))

(fn ReverseVertical
  (bind _returnvalue (Transformation|GetVelocity))
  (bind (_x _y _z) (Math|Vector|BreakVector _returnvalue))
  (if (>= (Variables|Default|GettimeSinceReversed) 0.0)
    (Variables|/Script/Engine.MovementComponent|SetVelocity (Variables|Default|GetProjectileMovement) (Math|Vector|MakeVector _x _y (* -1 _z)))
    (Variables|Default|SettimeSinceReversed 0.0)))