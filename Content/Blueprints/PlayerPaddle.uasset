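; PlayerPaddle is the player's paddle, moved vertically by an input axis and reacting to TheBall.
; Each tick it tests its X location against two limits, snapping Z to a fixed height above either one.
; Only at or below the lower X limit does it apply input-scaled movement and store MoveDirection.
; When its Box overlaps TheBall, it spawns an Invisableball at the ball's transform.
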(event OnComponentBeginOverlap(Box)
  (params (OverlappedComponent :type Primitive%20Component%20Object%20Reference) (OtherActor :type Actor%20Object%20Reference) (OtherComp :type Primitive%20Component%20Object%20Reference) (OtherBodyIndex :type Integer) (bFromSweep :type Boolean) (SweepResult :type Hit%20Result%20Structure%20%28by%20ref%29))
  (Utilities|Casting|CastToTheBall OtherActor)
  (Game|SpawnActorfromClass "/Game/Blueprints/Invisableball.Invisableball_C" (Transformation|GetActorTransform OtherActor) "Undefined" 0 0))

(event EventTick
  (params (DeltaSeconds :type Float%20%28single-precision%29))
  (bind _returnvalue (Transformation|GetActorLocation))
  (bind _returnvalue_2 (Transformation|GetActorLocation))
  (bind _returnvalue_3 (Input|AxisValues|Getverticalmovement))
  (bind (_x _y) (Math|Vector|BreakVector _returnvalue))
  (bind (_x_2 _y_2) (Math|Vector|BreakVector _returnvalue_2))
  (if (> (.X (Math|Vector|BreakVector (Transformation|GetActorLocation))) 15.0)
    (Transformation|SetActorLocation (Math|Vector|MakeVector _x_2 _y_2 14.0) false false)
    (elif (> (.X (Math|Vector|BreakVector (Transformation|GetActorLocation))) -15.0)
      (Transformation|SetActorLocation (Math|Vector|MakeVector _x _y -14.0) false false)
      (else
        (Transformation|AddActorLocalOffset (* (Math|Vector|MakeVector 0.0 0.0 (Variables|Default|GetMoveSpeed)) _returnvalue_3) false false)
        (Variables|Default|SetMoveDirection (Math|Float|Truncate _returnvalue_3))))))

(fn ConstructionScript)