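; EnemyPaddle2 is an AI-controlled paddle actor that follows the ball vertically.
; Each Tick it looks up the TheBall actor, stores its location, and SetDirection compares Z heights to choose up or down.
; It then moves one unit per frame on local Z without sweep or delta-time scaling, so speed depends on frame rate.
; The zero-direction branch is effectively unreachable because equal heights count as up.
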(event EventBeginPlay)

(event Collision|EventActorBeginOverlap
  (params (OtherActor :type Actor%20Object%20Reference)))

(event EventTick
  (params (DeltaSeconds :type Float%20%28single-precision%29))
  (bind _returnvalue (Actor|GetActorOfClass "/Game/Blueprints/TheBall.TheBall_C"))
  (Variables|Default|SettargetPosition (Transformation|GetActorLocation _returnvalue))
  (CallFunction|SetDirection)
  (Transformation|AddActorLocalOffset (Math|Vector|MakeVector 0.0 0.0 (Math|Conversions|ToFloat(Integer) (Variables|Default|GetMoveDirection))) false false))

(fn ConstructionScript)

(fn SetDirection
  (if (<= (.Z (Math|Vector|BreakVector (Transformation|GetActorLocation))) (.Z (Math|Vector|BreakVector (Variables|Default|GettargetPosition))))
    (Variables|Default|SetMoveDirection 1)
    (elif (>= (.Z (Math|Vector|BreakVector (Transformation|GetActorLocation))) (.Z (Math|Vector|BreakVector (Variables|Default|GettargetPosition))))
      (Variables|Default|SetMoveDirection -1)
      (else
        (Variables|Default|SetMoveDirection 0)))))